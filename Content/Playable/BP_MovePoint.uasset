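; BP_MovePoint is a hidden, clickable destination marker for moving BP_Playable or BP_Farmer.
; Pressing and releasing its mesh swaps materials, and release hides every move point if either character is in its Clicked state.
; The selected Playable jumps straight here and gets its cube material reset.
; The selected Farmer eases here through a timeline-driven lerp with an added vertical offset, and both paths clear the Clicked flags.
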(event `self.ReceiveBeginPlay`
  (`self.SetActorHiddenInGame` self true))

(event `self.ReceiveActorBeginOverlap`
  (params (OtherActor :type "Actor Object Reference")))

(event `self.StaticMesh.OnClicked`
  (params (TouchedComponent :type "PrimitiveComponent Object Reference") (ButtonPressed :type "Key Structure"))
  (`PrimitiveComponent.SetMaterial` TouchedComponent 0 "/Game/Material/MAT_Light3.MAT_Light3"))

(event `self.StaticMesh.OnReleased`
  (params (TouchedComponent :type "PrimitiveComponent Object Reference") (ButtonReleased :type "Key Structure"))
  (bind _playable (`self.Playable`))
  (set `self.Clicked` true)
  (`PrimitiveComponent.SetMaterial` TouchedComponent 0 "/Game/Material/MAT_Light2.MAT_Light2")
  (`|ExecutionSequence`
    (:`then_0`
      (bind _returnvalue (`GameplayStatics.GetActorOfClass` "/Game/Playable/BP_Playable.BP_Playable_C"))
      (set `self.Playable` _returnvalue)
      (if (`/Game/Playable/BP_Playable.Clicked` (`self.Playable`))
        (bind _outactors (`GameplayStatics.GetAllActorsOfClass` "BP_MovePoint_C"))
        (for _array_element _outactors
          (`self.SetActorHiddenInGame` _array_element true)
          (if (`self.Clicked`)
            (bind _output_get (set `self.MoveLocation` (`self.K2_GetActorLocation`)))
            (`self.K2_SetActorLocation` (`self.Playable`) _output_get false false)
            (set `self.Clicked` false)
            (set `/Game/Playable/BP_Playable.Clicked` false _playable)
            (`PrimitiveComponent.SetMaterial` (`/Game/Playable/BP_Playable.Cube` _playable) 0 "/Engine/BasicShapes/BasicShapeMaterial.BasicShapeMaterial")))))
    (:`then_1`
      (bind _returnvalue_2 (`GameplayStatics.GetActorOfClass` "/Game/Playable/BP_Farmer.BP_Farmer_C"))
      (set `self.Farmer` _returnvalue_2)
      (if (`/Game/Playable/BP_Farmer.Clicked` (`self.Farmer`))
        (bind _outactors_2 (`GameplayStatics.GetAllActorsOfClass` "BP_MovePoint_C"))
        (for _array_element_2 _outactors_2
          (`self.SetActorHiddenInGame` _array_element_2 true)
          (if (`self.Clicked`)
            (bind _output_get_2 (set `self.MoveLocation` (`self.K2_GetActorLocation`)))
            (bind (_direction _beta _alpha) (`Timeline|타임라인_0`)
              (:`Update`
                (`self.K2_SetActorLocation` (`self.Farmer`) (+ (`KismetMathLibrary.VLerp` (`self.K2_GetActorLocation` (`self.Farmer`)) _output_get_2 (* _alpha 0.1)) (`KismetMathLibrary.MakeVector` 0.0 0.0 (* _beta 10.0))) false false)
                (set `self.Clicked` false)
                (set `/Game/Playable/BP_Farmer.Clicked` false (`self.Farmer`))))))))))

(fn `UserConstructionScript`)