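; BP_Playable is a clickable cube actor that toggles a highlight when clicked.
; Each click calls Change, which flips the Clicked flag and swaps the cube's material between MAT_Light and BasicShapeMaterial.
; The click then tries to reveal a BP_MovePoint mesh, but the cast has no object connected, so that step never succeeds.
; The Show event is an empty stub.
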(event `self.ReceiveBeginPlay`
  (set `self.Clicked` false))

(event `self.Cube.OnClicked`
  (params (TouchedComponent :type "PrimitiveComponent Object Reference") (ButtonPressed :type "Key Structure"))
  (`self.Change`)
  (bind _asbp_move_point (cast `/Game/Playable/BP_MovePoint` _))
  (`SceneComponent.SetVisibility` (`/Game/Playable/BP_MovePoint.StaticMesh` _asbp_move_point) true false))

(event `Change`
  (if (`self.Clicked`)
    (`PrimitiveComponent.SetMaterial` (`self.Cube`) 0 "/Engine/BasicShapes/BasicShapeMaterial.BasicShapeMaterial")
    (set `self.Clicked` false)
    (else
      (`PrimitiveComponent.SetMaterial` (`self.Cube`) 0 "/Game/Playable/MAT_Light.MAT_Light")
      (set `self.Clicked` true))))

(event `Show`)

(fn `UserConstructionScript`)