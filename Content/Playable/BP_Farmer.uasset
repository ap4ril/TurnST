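; BP_Farmer is a playable farmer unit that toggles selection when its capsule is clicked and reveals nearby move points.
; Change swaps the skeletal mesh material between a highlight and a basic material while flipping the Clicked flag.
; The click handler then loops over all BP_MovePoint actors, showing those within a fixed horizontal range when selected and hiding all when deselected.
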(event `self.ReceiveBeginPlay`
  (set `self.Clicked` false))

(event `self.Capsule.OnClicked`
  (params (TouchedComponent :type "PrimitiveComponent Object Reference") (ButtonPressed :type "Key Structure"))
  (`self.Change`)
  (bind _outactors (`GameplayStatics.GetAllActorsOfClass` "/Game/Playable/BP_MovePoint.BP_MovePoint_C"))
  (for _array_element _outactors
    (if (`self.Clicked`)
      (if (<= (`self.GetHorizontalDistanceTo` _array_element) 200.0)
        (`self.SetActorHiddenInGame` _array_element false))
      (else
        (`self.SetActorHiddenInGame` _array_element true)))))

(event `Change`
  (if (`self.Clicked`)
    (`PrimitiveComponent.SetMaterial` (`self.SkeletalMesh`) 0 "/Engine/BasicShapes/BasicShapeMaterial.BasicShapeMaterial")
    (set `self.Clicked` false)
    (else
      (`PrimitiveComponent.SetMaterial` (`self.SkeletalMesh`) 0 "/Game/Material/MAT_Light.MAT_Light")
      (set `self.Clicked` true))))

(fn `UserConstructionScript`)